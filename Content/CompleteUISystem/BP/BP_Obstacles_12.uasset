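; BP_Obstacles_12 is an obstacle actor that damages the player and is tracked by compass and waypoint markers.
; After a short delay on BeginPlay, it creates a tinted compass marker widget bound to itself and sets its world waypoint widget's color.
; Tick sends the player distance in meters to the waypoint widget.
; Overlapping the HitBox subtracts a fixed amount from the ThirdPersonCharacter's Health.
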(event OnComponentBeginOverlap(HitBox)
  (params (OverlappedComponent :type Primitive%20Component%20Object%20Reference) (OtherActor :type Actor%20Object%20Reference) (OtherComp :type Primitive%20Component%20Object%20Reference) (OtherBodyIndex :type Integer) (bFromSweep :type Boolean) (SweepResult :type Hit%20Result%20Structure%20%28by%20ref%29))
  ;[1 1 1] Damage Health
  (bind _asthird_person_character (Utilities|Casting|CastToThirdPersonCharacter OtherActor))
  (Variables|/Game/CompleteUISystem/ThirdPersonBP/Blueprints/ThirdPersonCharacter.ThirdPersonCharacter_C|SetHealth _asthird_person_character (- (Variables|/Game/CompleteUISystem/ThirdPersonBP/Blueprints/ThirdPersonCharacter.ThirdPersonCharacter_C|GetHealth _asthird_person_character) 0.1)))

(event EventBeginPlay
  ;[1 1 1] Set the HitBox Marker and the Waypoint Marker color
  (|CompassSetUp)
  (Class|BPIMarkerWidget12|SetMarkerColor(Message) (UserInterface|GetUserWidgetObject (Variables|Default|GetMarkerWidget)) "(R=1.000000,G=1.000000,B=1.000000,A=1.000000)"))

(event EventTick
  (params (DeltaSeconds :type Float%20%28single-precision%29))
  ;[1 1 1] Calculate the distance to the object - Waypoint Marker
  (Class|BPIMarkerWidget12|UpdateDistance(Message) (UserInterface|GetUserWidgetObject (Variables|Default|GetMarkerWidget)) (Utilities|Text|ToText(String) (Utilities|String|Append (Utilities|String|ToString(Integer) (Math|Float|Truncate (/ (Math|Vector|Distance(Vector) (Transformation|GetActorLocation) (Transformation|GetActorLocation (Game|GetPlayerCharacter 0))) 1e+02))) "m"))))

(fn ConstructionScript)