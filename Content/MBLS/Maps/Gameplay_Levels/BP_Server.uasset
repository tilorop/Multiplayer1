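; BP_Server is a level actor that gathers references to the game mode and players at startup.
; On BeginPlay it sets a test string, then runs custom events that find the first BP_GM_Base actor and copy its AllPCs list into Playarray.
; Its server-reference event finds the first BP_Server but assigns None to that actor's ServerRef, so no self-reference is stored.
; Tick, overlap and construction logic are empty.
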(event Custom|bp_server_ref
  ;[1 1 1] bp_server reference
  (bind _outactors (Actor|GetAllActorsOfClass "BP_Server_C"))
  (Variables|BP_Server_C|SetServerRef (Utilities|Array|Get(acopy) _outactors) 0))

(event Custom|player_array
  ;[1 1 1] Adder spillere til playarray
  (Variables|Default|Setplayarray (Variables|/Game/MBLS/Blueprints/Core/Base/Core/BP_GM_Base.BP_GM_Base_C|GetAll_PC's (Variables|Default|GetGMbase))))

(event Custom|GMbase_ref
  ;[1 1 1] GMbase reference
  (bind _outactors (Actor|GetAllActorsOfClass "/Game/MBLS/Blueprints/Core/Base/Core/BP_GM_Base.BP_GM_Base_C"))
  (Variables|Default|SetGMbase (Utilities|Array|Get(acopy) _outactors)))

(event EventBeginPlay
  ;[1 1 1] Starter opp ting, og setter  variabler, arrays etc
  (Variables|Default|Setteststring "Jallajalla")
  (CallFunction|BpServerRef)
  (CallFunction|GMbaseRef)
  (CallFunction|PlayerArray))

(event Collision|EventActorBeginOverlap
  (params (OtherActor :type Actor%20Object%20Reference))
  ;[1 1 1] Comment
)

(event EventTick
  (params (DeltaSeconds :type Float%20%28single-precision%29))
  ;[1 1 1] Comment
)

(fn ConstructionScript)